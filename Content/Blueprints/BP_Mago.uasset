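; BP_Mago is a mage Blueprint that prints its stats and frame timing as on-screen debug text.
; BeginPlay builds one message from the name, health, damage and spell count variables, shown for a variable-set duration.
; Tick prints delta seconds and a GetFramePace value labeled FPS, using a fixed key so the line updates in place.
; The construction script is empty, and the graphs contain no gameplay logic.
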(event `self.ReceiveBeginPlay`
  (`KismetSystemLibrary.PrintString` (`KismetStringLibrary.Concat_StrStr` "Nombre: " (`self.NombreMago`) " \nVida Actual: " (`KismetStringLibrary.Conv_DoubleToString` (`self.Vida`)) " \nDaño:  " (`KismetStringLibrary.Conv_DoubleToString` (`self.Daño`)) " \nCantidad de Hechizos: " (`KismetStringLibrary.Conv_IntToString` (`self.Hechizos`))) true true (struct :`R` 0.079539 :`G` 1.0 :`A` 1.0) (`self.DuraciondeMensaje`)))

(event `self.ReceiveTick`
  (params (DeltaSeconds :type "Float (single-precision)"))
  (`KismetSystemLibrary.PrintString` (`KismetStringLibrary.Concat_StrStr` " \nDelta Seconds: " (`KismetStringLibrary.Conv_DoubleToString` DeltaSeconds) " \nFPS: " (`KismetStringLibrary.Conv_IntToString` (`GameUserSettings.GetFramePace`))) true true (struct :`G` 1.0 :`B` 0.039802 :`A` 1.0) 2.0 "1"))

(fn `UserConstructionScript`)