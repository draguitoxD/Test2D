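; BP_STBE is a small demo Blueprint of Set Timer by Event that heals a character over time.
; BeginPlay starts a looping timer bound to the CurarPersonaje event, firing every TicksCuracion seconds.
; Each tick adds a fixed amount to Vida and prints it, until a tick finds Vida at or above VidaMax and clears the timer by function name rather than by handle.
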(event `self.ReceiveBeginPlay`
  (`KismetSystemLibrary.K2_SetTimerDelegate` (delegate `CurarPersonaje`) (`self.ticksCuracion`) true)
  (`KismetSystemLibrary.PrintString` "Next" true true (struct :`R` 1.0 :`G` 0.978938 :`A` 1.0) 60.0))

(event `CurarPersonaje`
  (if (>= (`self.vida`) (`self.vidaMax`))
    (`KismetSystemLibrary.K2_ClearTimer` null "CurarPersonaje")
    (`KismetSystemLibrary.PrintString` "Clear" true true (struct :`R` 1.0 :`G` 0.37499 :`A` 1.0) 10.0)
    (else
      (bind _output_get (set `self.vida` (+ (`self.vida`) 10.0)))
      (`KismetSystemLibrary.PrintString` (`KismetStringLibrary.Concat_StrStr` "CURACION \nLa vida de tu personaje es: " (`KismetStringLibrary.Conv_DoubleToString` _output_get)) true true (struct :`G` 1.0 :`B` 0.672905 :`A` 1.0) 100.0))))

(fn `UserConstructionScript`)