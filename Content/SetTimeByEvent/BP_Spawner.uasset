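; BP_Spawner is an actor that repeatedly spawns projectiles or boost actors at its own transform.
; BeginPlay starts a looping Set Timer by Event at the SpawnTick interval, firing SpawnProyectil.
; That event branches on flags: Boost with SuperBoost spawns BP_SuperBoost, Boost alone spawns BP_Boost, otherwise BP_Proyectil spawns, with PRapida multiplying its velocity.
; Each branch prints a debug string naming the shot type.
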(event `self.ReceiveBeginPlay`
  (`KismetSystemLibrary.K2_SetTimerDelegate` (delegate `SpawnProyectil`) (`self.SpawnTick`) true))

(event `SpawnProyectil`
  (if (and (`self.bBoost?`) (`self.bSuperBoost?`))
    (`|SpawnActorFromClass` "/Game/SetTimeByEvent/BP_SuperBoost.BP_SuperBoost_C" (`self.GetTransform`) "Undefined" "MultiplyWithRoot" null null)
    (`KismetSystemLibrary.PrintString` "SUPER BOOST!!" true true (struct :`R` 1.0 :`G` 0.580053 :`A` 1.0))
    (elif (`self.bBoost?`)
      (`|SpawnActorFromClass` "/Game/SetTimeByEvent/BP_Boost.BP_Boost_C" (`self.GetTransform`) "Undefined" "MultiplyWithRoot" null null)
      (`KismetSystemLibrary.PrintString` "Boost!" true true (struct :`R` 1.0 :`G` 0.202704 :`A` 1.0))
      (elif (`self.bPRapida?`)
        (`|SpawnActorFromClass` "/Game/SetTimeByEvent/BP_Proyectil.BP_Proyectil_C" (`self.GetTransform`) "Undefined" "MultiplyWithRoot" null (* (`self.VelocidadP`) 10.0) null)
        (`KismetSystemLibrary.PrintString` "Rapid Fire!!" true true (struct :`R` 0.574428 :`B` 1.0 :`A` 1.0))
        (else
          (`|SpawnActorFromClass` "/Game/SetTimeByEvent/BP_Proyectil.BP_Proyectil_C" (`self.GetTransform`) "Undefined" "MultiplyWithRoot" null (`self.VelocidadP`) null)
          (`KismetSystemLibrary.PrintString` "shoot!!" true true (struct :`R` 1.0 :`B` 0.054783 :`A` 1.0)))))))

(fn `UserConstructionScript`)