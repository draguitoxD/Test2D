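; Practice Blueprint for math operators, functions and conditionals that simulates a character losing health until death.
; On BeginPlay it loops every two seconds while health is above zero, calling HacerDaño to subtract damage and MostrarVida to print the remaining health.
; When health runs out it prints a death message.
; Disconnected example chains print arithmetic results, call SumarDosNumeros and branch on a boolean, but never execute.
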(event `self.ReceiveBeginPlay`
  (if (> (`self.vidaPersonaje`) 0.0) :!label _label
    (`self.HacerDaño` (`self.daño`) (`self.vidaPersonaje`))
    (`self.MostrarVida` (`self.vidaPersonaje`))
    (`KismetSystemLibrary.Delay` 2.0)
    (goto _label)
    (else
      (`KismetSystemLibrary.PrintString` "Has muerto" true true (struct :`R` 1.0 :`G` 0.119454 :`A` 1.0) 100.0))))

(fn `HacerDaño`
  (params (`daño` :type "Float (double-precision)") (vida :type "Float (double-precision)"))
  (set `self.vidaPersonaje` (- vida `daño`)))

(fn `MostrarVida`
  (params (num :type "Float (double-precision)"))
  (`KismetSystemLibrary.PrintString` (`KismetStringLibrary.Concat_StrStr` "La Vida de tu personaje es: " (`KismetStringLibrary.Conv_DoubleToString` num)) true true (struct :`G` 1.0 :`B` 0.430231 :`A` 1.0) 100.0))

(fn `SumarDosNumeros`
  (params (num1 :type "Float (double-precision)") (num2 :type "Float (double-precision)"))
  (returns (resultado :type "Float (double-precision)"))
  (return (+ num1 num2)))

(fn `UserConstructionScript`)